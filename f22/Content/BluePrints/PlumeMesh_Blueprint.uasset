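; Engine plume mesh actor for the player's F22 jet, with a visual strength that follows the aircraft's speed.
; On BeginPlay it snaps its mesh onto the F22 pawn's PlaneMesh and creates a dynamic instance of the engine plume material.
; Every Tick it feeds the pawn's raw velocity magnitude into that material's PlumeStrength parameter.
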(event `self.ReceiveBeginPlay`
  (bind _asf_22pawn (cast `f22Pawn` (`GameplayStatics.GetPlayerPawn` 0)))
  (`SceneComponent.K2_AttachToComponent` (`self.StaticMeshComponent`) (`f22Pawn.PlaneMesh` _asf_22pawn) "None" "SnapToTarget" "SnapToTarget" "SnapToTarget" true)
  (set `self.PlayerPawn` _asf_22pawn)
  (`self.EnginePlumeSetup`))

(event `self.ReceiveTick`
  (params (DeltaSeconds :type "Float (single-precision)"))
  (`self.PawnUpdatematerial`))

(event `EnginePlumeSetup`
  (bind _staticmeshcomponent (`self.StaticMeshComponent`))
  (bind _returnvalue (`PrimitiveComponent.CreateDynamicMaterialInstance` _staticmeshcomponent 0 "/Game/Flying/Meshes/EnginePlumeMaterial_Inst.EnginePlumeMaterial_Inst" "None"))
  (bind _output_get (set `self.MaterialRef` _returnvalue))
  (`PrimitiveComponent.SetMaterial` _staticmeshcomponent 0 _output_get))

(event `Update Material Values`
  (params (Value :type "Float (double-precision)"))
  (bind _materialref (`self.MaterialRef`))
  (`/Engine/EditorBlueprintResources/StandardMacros.IsValid` _materialref
    (:`Is Valid`
      (`MaterialInstanceDynamic.SetScalarParameterValue` _materialref "PlumeStrength" Value))))

(event `PawnUpdatematerial`
  (`self.Update Material Values` (`KismetMathLibrary.VSize` (`self.GetVelocity` (`self.PlayerPawn`)))))

(fn `UserConstructionScript`)